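; Projectile actor for the Vaqueros game that destroys EnemyBP and ZombieBP actors it overlaps.
; An EnemyBP hit also calls CreateLootBox and destroys the projectile, while a ZombieBP hit leaves the projectile alive and drops no loot.
; CreateLootBox uses a weighted random roll to usually spawn an ammo LootBoxBP at the projectile Cube's X and Y, leaving Z unset.
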(event Custom|CreateLootBox
  (bind _cube (Variables|Default|GetCube))
  (bind _returnvalue (Transformation|GetWorldTransform _cube))
  ;[1 1 1] Crear caja de munición
  (if (Math|Random|RandomBoolwithWeight 0.85)
    (Game|SpawnActorfromClass "/Game/Vaqueros/AmmunitionBox/LootBoxBP.LootBoxBP_C" (Math|Transform|MakeTransform (Math|Vector|MakeVector (.x (.location _returnvalue)) (.y (.location _returnvalue)) 0.0) "0, 0, 0" "1,1,1") "Undefined" 0 0)))

(event Collision|EventActorBeginOverlap
  (params (OtherActor :type Actor%20Object%20Reference))
  ;[1 1 1] Colisión con enemigos
  (bind _asenemy_bp (Utilities|Casting|CastToEnemyBP OtherActor)
    (:then
      (Actor|DestroyActor _asenemy_bp)
      (CallFunction|CreateLootBox)
      (Actor|DestroyActor))
    (:CastFailed
      (bind _aszombie_bp (Utilities|Casting|CastToZombieBP OtherActor))
      (Actor|DestroyActor _aszombie_bp))))

(fn ConstructionScript)