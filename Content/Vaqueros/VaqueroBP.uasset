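; VaqueroBP is a playable cowboy character with twin-stick controls, jumping and a shotgun.
; Movement follows world X/Y axes, while separate direction axes build a vector that sets player 0's control rotation for aiming.
; Shooting plays a shotgun sound and spawns ProjectileBP from three direction components, each projectile consuming one from the Shoots ammo count.
; A DoOnce reset after a delay enforces the cooldown between volleys.
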(event Custom|ShootFromArrows
  ;[1 1 1] Shoot
  (Utilities|FlowControl|DoOnce false :!label _label
    (:Completed
      (if (> (Variables|Default|GetShoots) 0)
        (Audio|PlaySound2D "/Game/Vaqueros/escopeta_Cue.escopeta_Cue")
        (CallFunction|Shoot (Transformation|GetWorldTransform (Variables|Default|GetShootDirection)))
        (CallFunction|Shoot (Transformation|GetWorldTransform (Variables|Default|GetShootDirection1)))
        (CallFunction|Shoot (Transformation|GetWorldTransform (Variables|Default|GetShootDirection2)))
        (Utilities|FlowControl|Delay 1.0)
        (goto _label Reset)
        (else
          (goto _label Reset))))))

(event Custom|Shoot
  (params (Spawn%20Transform :type Transform))
  ;[1 1 1] Shoot
  (if (> (Variables|Default|GetShoots) 0)
    (Game|SpawnActorfromClass "/Game/Vaqueros/ProjectileBP.ProjectileBP_C" Spawn%20Transform "Undefined" 0 0)
    (Variables|Default|SetShoots (- (Variables|Default|GetShoots) 1))))

(event Input|ActionEvents|InputActionShoot
  (params (Key :type Key%20Structure :default "AnyKey"))
  ;[1 1 1] Shoot
  (:Pressed
    (CallFunction|ShootfromArrows)))

(event Input|ActionEvents|InputActionJump
  (params (Key :type Key%20Structure :default "AnyKey"))
  (:Pressed
    (Character|Jump)))

(event Input|AxisEvents|InputAxisMoveRightLeft
  (params (AxisValue :type Float%20%28single-precision%29))
  ;[1 0.07 0.07] Movement
  (Pawn|Input|AddMovementInput "0.000000,1.000000, 0" AxisValue false))

(event Input|AxisEvents|InputAxisDirectionUpDown
  (params (AxisValue :type Float%20%28single-precision%29))
  ;[0.3152 0.7012 1] Rotation
  (bind _output_get (Variables|Default|SetDirectionVector (Math|Vector|MakeVector AxisValue (.y (Variables|Default|GetDirectionVector)) 0.0)))
  (if (Math|Vector|NotEqual(Vector) _output_get "0, 0, 0" 0.0001)
    (Pawn|SetControlRotation (Game|GetPlayerController 0) (Math|Conversions|RotationFromXVector _output_get))))

(event Input|AxisEvents|InputAxisDirectionRightLeft
  (params (AxisValue :type Float%20%28single-precision%29))
  ;[0.3152 0.7012 1] Rotation
  (bind _output_get (Variables|Default|SetDirectionVector (Math|Vector|MakeVector (.x (Variables|Default|GetDirectionVector)) AxisValue 0.0)))
  (if (Math|Vector|NotEqual(Vector) _output_get "0, 0, 0" 0.0001)
    (Pawn|SetControlRotation (Game|GetPlayerController 0) (Math|Conversions|RotationFromXVector _output_get))))

(event Input|AxisEvents|InputAxisMoveUpDown
  (params (AxisValue :type Float%20%28single-precision%29))
  ;[1 0.07 0.07] Movement
  (Pawn|Input|AddMovementInput "1.000000,0.000000, 0" AxisValue false))

(fn ConstructionScript)